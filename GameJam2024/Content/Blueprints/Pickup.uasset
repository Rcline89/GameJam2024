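; Pickup actor that floats and spins, shows a click icon for the clown character, and reports back to its owning PickupLocation for respawning.
; Construction script picks the mesh from the PickupList data table by PickupType.
; Timelines drive idle motion, icon scaling on overlap or drop, and a scale-and-shake kill before destruction, with VFX still a print placeholder.
; First pickup and kill each tell the location to ready another spawn.
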(event `self.ReceiveBeginPlay`
  (bind (_returnvalue_x _returnvalue_y _returnvalue_z) (`KismetMathLibrary.BreakVector` (`self.K2_GetActorLocation`)))
  (bind _pickupmesh (`self.PickupMesh`))
  (bind _aspickup_location (cast `/Game/Blueprints/PickupLocation` (`self.GetOwner`))
    (:`then`
      (set `self.OwnerLocation` _aspickup_location))
    (:`CastFailed`
      _))
  (set `self.InitialLocation` (`self.K2_GetActorLocation`))
  (bind (_direction _float _spin) (`Timeline|FloatAndSpinTimeline` :!via `PlayFromStart`)
    (:`Update`
      (`SceneComponent.K2_SetWorldRotation` _pickupmesh (`KismetMathLibrary.MakeRotator` 0.0 0.0 (* _spin 360.0)) false false)
      (`SceneComponent.K2_SetWorldLocation` _pickupmesh (`KismetMathLibrary.MakeVector` _returnvalue_x _returnvalue_y (+ _returnvalue_z (* _float 10.0))) false false))))

(event `Dropped`
  (set `self.InitialLocation` (`self.K2_GetActorLocation`))
  (`TimelineComponent.Play` (`self.FloatAndSpinTimeline`))
  (`SceneComponent.SetHiddenInGame` (`self.ClickIcon`) false false :!label _label)
  (bind (_direction _progress) (`Timeline|ClickIconTimeline` :!via `PlayFromStart` :!label _label_2)
    (:`Update`
      (`SceneComponent.SetWorldScale3D` (`self.ClickIcon`) (`KismetMathLibrary.Conv_DoubleToVector` _progress)))
    (:`Finished`
      (switch `ETimelineDirection` _direction
        (:`Backward`
          (`SceneComponent.SetHiddenInGame` (`self.ClickIcon`) true false))))))

(event `self.ReceiveActorBeginOverlap`
  (params (OtherActor :type "Actor Object Reference"))
  (cast `/Game/Blueprints/ClownCharacter` OtherActor)
  (goto _label))

(event `self.ReceiveActorEndOverlap`
  (params (OtherActor :type "Actor Object Reference"))
  (cast `/Game/Blueprints/ClownCharacter` OtherActor)
  (goto _label_2 :!via `ReverseFromEnd`))

(event `PickedUp`
  (`TimelineComponent.Stop` (`self.FloatAndSpinTimeline`))
  (`SceneComponent.SetHiddenInGame` (`self.ClickIcon`) true false)
  (`/Engine/EditorBlueprintResources/StandardMacros.DoOnce` false
    (:`Completed`
      (`/Game/Blueprints/PickupLocation.ReadyToSpawnAnother` (`self.OwnerLocation`)))))

(event `KillItem`
  (set `self.SetToKill` true)
  (`TimelineComponent.Stop` (`self.FloatAndSpinTimeline`))
  (bind (_direction _scale _shakeamount) (`Timeline|KillItemTimeline` :!via `PlayFromStart`)
    (:`Update`
      (`self.SetActorScale3D` (`KismetMathLibrary.Conv_DoubleToVector` _scale))
      (bind _returnvalue (* _shakeamount 10.0))
      (`self.K2_AddActorLocalRotation` (`KismetMathLibrary.MakeRotator` _returnvalue _returnvalue _returnvalue)))
    (:`Finished`
      (`KismetSystemLibrary.PrintString` "Play VFX")
      (`/Game/Blueprints/PickupLocation.ReadyToSpawnAnother` (`self.OwnerLocation`))
      (`self.K2_DestroyActor`))))

(fn `UserConstructionScript`
  (bind _outrownames (`DataTableFunctionLibrary.GetDataTableRowNames` "/Game/Blueprints/Misc/PickupList.PickupList"))
  (for _array_element _outrownames
    (bind _returnvalue (`|GetDataTableRow` "/Game/Blueprints/Misc/PickupList.PickupList" _array_element)
      (:`then`
        (bind (_mesh _name) (break `/Game/Blueprints/Misc/PickupStruct` _returnvalue))
        (if (`|EnumEquality` _name (`self.PickupType`))
          (`StaticMeshComponent.SetStaticMesh` (`self.PickupMesh`) _mesh))))))