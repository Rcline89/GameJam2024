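; HumanObstacle is an obstacle actor whose human collision component travels along a spline path.
; On BeginPlay it sets the RunTheLoop timeline's play rate from spline length and Speed, then plays it from the start.
; Each timeline update maps Progress to a distance along PathSpline and applies that world-space location and rotation to HumanCollision.
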(event `self.ReceiveBeginPlay`
  (bind _pathspline (`self.PathSpline`))
  (`TimelineComponent.SetPlayRate` (`self.RunTheLoop`) (/ 1.0 (/ (`SplineComponent.GetSplineLength` (`self.PathSpline`)) (`self.Speed`))))
  (bind (_direction _progress) (`Timeline|RunTheLoop` :!via `PlayFromStart`)
    (:`Update`
      (bind (_returnvalue_location _returnvalue_rotation) (`KismetMathLibrary.BreakTransform` (`SplineComponent.GetTransformAtDistanceAlongSpline` _pathspline (`KismetMathLibrary.Lerp` 0.0 (`SplineComponent.GetSplineLength` _pathspline) _progress) "World" false)))
      (`SceneComponent.K2_SetWorldLocationAndRotation` (`self.HumanCollision`) _returnvalue_location _returnvalue_rotation false false))))

(fn `UserConstructionScript`)